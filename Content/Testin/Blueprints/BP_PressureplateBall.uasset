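; BP_PressureplateBall is a physics ball, apparently for pressure plate puzzles, that returns to its starting point when it hits a reset or death volume.
; BeginPlay stores the start location, and the mesh's begin-overlap event checks for BP_Deathtrigger_Test or BP_BallReset actors.
; Either match calls ResetPos, which moves the ball back without sweep or teleport and zeroes its linear velocity, leaving rotation and angular velocity untouched.
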(event `self.ReceiveBeginPlay`
  (set `self._startPos` (`self.K2_GetActorLocation`)))

(event `self.Mesh.OnComponentBeginOverlap`
  (params (OverlappedComponent :type "PrimitiveComponent Object Reference") (OtherActor :type "Actor Object Reference") (OtherComp :type "PrimitiveComponent Object Reference") (OtherBodyIndex :type Integer) (bFromSweep :type Boolean) (SweepResult :type "HitResult Structure (by ref)"))
  (cast `/Game/Testin/Blueprints/BP_Deathtrigger_Test` OtherActor
    (:`then`
      _)
    (:`CastFailed`
      (cast `/Game/Testin/Blueprints/BP_BallReset` OtherActor)))
  (`self.ResetPos`))

(fn `ResetPos`
  (`self.K2_SetActorLocation` (`self._startPos`))
  (`PrimitiveComponent.SetPhysicsLinearVelocity` (`self.Mesh`) (0.0 0.0 0.0) false "None"))

(fn `UserConstructionScript`)