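; BP_PauseHandler is an input-enabled Blueprint that opens and closes the pause menu widget.
; The Pause and Open Skilltree actions toggle WBP_PauseMenu, passing it a handler reference, while the gamepad right face button removes it.
; Opening calls SwapToUI to show the cursor, set Game and UI input, and disable character input; closing here does not revert this.
; D-pad up/down select between two menu buttons, and the bottom face button clicks the selection.
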(event `self.ReceiveBeginPlay`
  (`self.EnableInput` (`GameplayStatics.GetPlayerController` 0)))

(event `InputAction|Pause` :consume false
  (params (Key :type "Key Structure"))
  (bind _pausemenu (`self.PauseMenu`))
  (:`Pressed`
    (`/Engine/EditorBlueprintResources/StandardMacros.IsValid` _pausemenu :!label _label
      (:`Is Valid`
        (`Widget.RemoveFromParent` _pausemenu :!label _label_2)
        (set `self.PauseMenu` null))
      (:`Is Not Valid`
        (bind _returnvalue (`|CreateWidget` "/Game/Testin/Blueprints/UI/WBP_PauseMenu.WBP_PauseMenu_C" null self))
        (bind _output_get (set `self.PauseMenu` _returnvalue))
        (`UserWidget.AddToViewport` _output_get 0)
        (`self.SwapToUI`)))))

(event `Key|Gamepad_FaceButton_Right` :consume false
  (params (Key :type "Key Structure"))
  (:`Pressed`
    (goto _label_2)))

(event `InputAction|Open Skilltree` :consume false
  (params (Key :type "Key Structure"))
  (:`Pressed`
    (goto _label)))

(event `Key|Gamepad_DPad_Up` :consume false
  (params (Key :type "Key Structure"))
  (bind _pausemenu (`self.PauseMenu`))
  (:`Pressed`
    (`/Engine/EditorBlueprintResources/StandardMacros.IsValid` (`self.PauseMenu`)
      (:`Is Valid`
        (set `/Game/Testin/Blueprints/UI/WBP_PauseMenu._currentSelectedButton` (`/Game/Testin/Blueprints/UI/WBP_PauseMenu.Button_0` _pausemenu) _pausemenu)))))

(event `Key|Gamepad_DPad_Down` :consume false
  (params (Key :type "Key Structure"))
  (bind _pausemenu (`self.PauseMenu`))
  (:`Pressed`
    (`/Engine/EditorBlueprintResources/StandardMacros.IsValid` (`self.PauseMenu`)
      (:`Is Valid`
        (set `/Game/Testin/Blueprints/UI/WBP_PauseMenu._currentSelectedButton` (`/Game/Testin/Blueprints/UI/WBP_PauseMenu.Button` _pausemenu) _pausemenu)))))

(event `Key|Gamepad_FaceButton_Bottom` :consume false
  (params (Key :type "Key Structure"))
  (bind _pausemenu (`self.PauseMenu`))
  (:`Pressed`
    (`/Engine/EditorBlueprintResources/StandardMacros.IsValid` _pausemenu
      (:`Is Valid`
        (`/Game/Testin/Blueprints/UI/WBP_PauseMenu.ClickSelected` _pausemenu)))))

(fn `SwapToUI`
  (bind _returnvalue (`GameplayStatics.GetPlayerController` 0))
  (set `PlayerController.bShowMouseCursor` true _returnvalue)
  (`WidgetBlueprintLibrary.SetInputMode_GameAndUIEx` _returnvalue null)
  (`self.DisableInput` (`GameplayStatics.GetPlayerCharacter` 0) _returnvalue))

(fn `UserConstructionScript`)