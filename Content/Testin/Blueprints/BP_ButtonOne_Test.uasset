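; Test button actor that moves a referenced Platform actor toward a Destination actor while the player holds Interact within its trigger box.
; Box overlaps with BP_Character_Test gate the input, which is enabled for player 0 on BeginPlay.
; Tick moves the platform at PlatformSpeed with interpolated rotation, stopping within a small distance of the target.
; Releasing Interact or leaving the box sends it back toward its cached starting transform.
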(event `self.ReceiveBeginPlay`
  (bind _platform (`self.platform`))
  (`self.EnableInput` (`GameplayStatics.GetPlayerController` 0))
  (set `self._startPos` (`self.K2_GetActorLocation` _platform))
  (set `self._startRot` (`self.K2_GetActorRotation` _platform)))

(event `self.ReceiveTick`
  (params (DeltaSeconds :type "Float (single-precision)"))
  (bind _platform (`self.platform`))
  (bind _platform_2 (`self.platform`))
  (bind _platform_3 (`self.platform`))
  (bind _destination (`self.destination`))
  (bind _platform_4 (`self.platform`))
  (bind (_returnvalue_location _returnvalue_rotation _returnvalue_scale) (`KismetMathLibrary.BreakTransform` (`self.GetTransform` _platform)))
  (bind (_returnvalue_location_2 _returnvalue_rotation_2 _returnvalue_scale_2) (`KismetMathLibrary.BreakTransform` (`self.GetTransform` _platform_4)))
  (if (and (`self.hasBeenPressed`) (`self._canBePressed`))
    (if (not (< (`KismetMathLibrary.VSize` (- (`self.K2_GetActorLocation` (`self.destination`)) (`self.K2_GetActorLocation` (`self.platform`)))) 10.0))
      (`self.K2_SetActorTransform` _platform (`KismetMathLibrary.MakeTransform` (+ _returnvalue_location (* (`KismetMathLibrary.Normal` (- (`self.K2_GetActorLocation` _destination) (`self.K2_GetActorLocation` _platform_2))) (* (`GameplayStatics.GetWorldDeltaSeconds`) (`self.platformSpeed`)))) (`KismetMathLibrary.RInterpTo` (`self.K2_GetActorRotation` _platform_2) (`self.K2_GetActorRotation` _destination) (`GameplayStatics.GetWorldDeltaSeconds`) 1.0) _returnvalue_scale) false false))
    (elif (not (< (`KismetMathLibrary.VSize` (- (`self._startPos`) (`self.K2_GetActorLocation` (`self.platform`)))) 10.0))
      (`self.K2_SetActorTransform` _platform_4 (`KismetMathLibrary.MakeTransform` (+ _returnvalue_location_2 (* (`KismetMathLibrary.Normal` (- (`self._startPos`) (`self.K2_GetActorLocation` _platform_3))) (* (`GameplayStatics.GetWorldDeltaSeconds`) (`self.platformSpeed`)))) (`KismetMathLibrary.RInterpTo` (`self.K2_GetActorRotation` _platform_3) (`self._startRot`) (`GameplayStatics.GetWorldDeltaSeconds`) 1.0) _returnvalue_scale_2) false false))))

(event `self.Box.OnComponentBeginOverlap`
  (params (OverlappedComponent :type "PrimitiveComponent Object Reference") (OtherActor :type "Actor Object Reference") (OtherComp :type "PrimitiveComponent Object Reference") (OtherBodyIndex :type Integer) (bFromSweep :type Boolean) (SweepResult :type "HitResult Structure (by ref)"))
  (cast `/Game/Testin/BP_Character_Test` OtherActor)
  (set `self._canBePressed` true))

(event `self.Box.OnComponentEndOverlap`
  (params (OverlappedComponent :type "PrimitiveComponent Object Reference") (OtherActor :type "Actor Object Reference") (OtherComp :type "PrimitiveComponent Object Reference") (OtherBodyIndex :type Integer))
  (cast `/Game/Testin/BP_Character_Test` OtherActor)
  (set `self._canBePressed` false))

(event `InputAction|Interact` :consume false
  (params (Key :type "Key Structure"))
  (:`Pressed`
    (if (`self._canBePressed`)
      (set `self.hasBeenPressed` true)))
  (:`Released`
    (set `self.hasBeenPressed` false)))

(fn `UserConstructionScript`)