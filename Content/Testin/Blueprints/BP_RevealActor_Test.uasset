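; BP_RevealActor_Test is a test actor that turns itself off five seconds after leaving a BP_Gadget_Test reveal sphere.
; Begin overlap with that sphere cancels and resets the countdown; end overlap starts it, gated by CanEndOverlap.
; A Tick timer then sets the mesh to ignore WorldStatic and GameTraceChannel1 and deactivates VFX.
; The graph contains no logic that re-enables collision or VFX.
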(event `self.ReceiveTick`
  (params (DeltaSeconds :type "Float (single-precision)"))
  (bind __timer (`self._timer`))
  (bind _staticmeshcomponent (`self.StaticMeshComponent`))
  (if (`self._startCountdown`)
    (set `self._timer` (+ __timer (`GameplayStatics.GetWorldDeltaSeconds`)))
    (if (>= __timer 5.0)
      (`PrimitiveComponent.SetCollisionResponseToChannel` _staticmeshcomponent "ECC_GameTraceChannel1" "ECR_Ignore")
      (`PrimitiveComponent.SetCollisionResponseToChannel` _staticmeshcomponent "ECC_WorldStatic" "ECR_Ignore")
      (`ActorComponent.Deactivate` (`self.VFX`))
      (set `self._startCountdown` false)
      (set `self._timer` 0.0)
      (set `self._canEndOverlap` false))))

(event `self.StaticMeshComponent.OnComponentEndOverlap`
  (params (OverlappedComponent :type "PrimitiveComponent Object Reference") (OtherActor :type "Actor Object Reference") (OtherComp :type "PrimitiveComponent Object Reference") (OtherBodyIndex :type Integer))
  (bind _asbp_gadget_test (cast `/Game/Testin/Blueprints/BP_Gadget_Test` OtherActor))
  (if (and (== (`/Game/Testin/Blueprints/BP_Gadget_Test.RevealSphere` _asbp_gadget_test) OtherComp) (`self._canEndOverlap`))
    (set `self._startCountdown` true)))

(event `self.StaticMeshComponent.OnComponentBeginOverlap`
  (params (OverlappedComponent :type "PrimitiveComponent Object Reference") (OtherActor :type "Actor Object Reference") (OtherComp :type "PrimitiveComponent Object Reference") (OtherBodyIndex :type Integer) (bFromSweep :type Boolean) (SweepResult :type "HitResult Structure (by ref)"))
  (bind _asbp_gadget_test (cast `/Game/Testin/Blueprints/BP_Gadget_Test` OtherActor))
  (if (== (`/Game/Testin/Blueprints/BP_Gadget_Test.RevealSphere` _asbp_gadget_test) OtherComp)
    (set `self._startCountdown` false)
    (set `self._timer` 0.0)
    (set `self._canEndOverlap` true)))

(fn `UserConstructionScript`)