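; Main menu handler actor that spawns WBP_MainMenu on BeginPlay, shows the cursor and adds gamepad navigation.
; D-pad presses set the widget's CurrentSelectedButton through a hard-coded layout, with Right choosing the Back button on Settings or Credits screens.
; Bottom face button calls the selected button's function; right face button backs out of Settings or Credits.
; Most inputs fetch the widget through MainMenuVisibleCheck, which tests that the main panel is visible.
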(event `self.ReceiveBeginPlay`
  (bind _returnvalue (`GameplayStatics.GetPlayerController` 0))
  (`self.EnableInput` (`GameplayStatics.GetPlayerController` 0))
  (bind _returnvalue_2 (`|CreateWidget` "/Game/Testin/Blueprints/UI/WBP_MainMenu.WBP_MainMenu_C"))
  (bind _output_get (set `self.MainMenu` _returnvalue_2))
  (`UserWidget.AddToViewport` _output_get 0)
  (`WidgetBlueprintLibrary.SetInputMode_GameAndUIEx` _returnvalue _returnvalue_2)
  (set `PlayerController.bShowMouseCursor` true _returnvalue))

(event `Key|Gamepad_DPad_Up`
  (params (Key :type "Key Structure"))
  (:`Pressed`
    (bind _outputpin (`self.MainMenuVisibleCheck`))
    (set `/Game/Testin/Blueprints/UI/WBP_MainMenu._currentSelectedButton` (`/Game/Testin/Blueprints/UI/WBP_MainMenu.NewGameButton` _outputpin) _outputpin)))

(event `Key|Gamepad_DPad_Down`
  (params (Key :type "Key Structure"))
  (:`Pressed`
    (bind _outputpin (`self.MainMenuVisibleCheck`))
    (if (== (`/Game/Testin/Blueprints/UI/WBP_MainMenu._currentSelectedButton` _outputpin) (`/Game/Testin/Blueprints/UI/WBP_MainMenu.CreditsButton` _outputpin))
      (set `/Game/Testin/Blueprints/UI/WBP_MainMenu._currentSelectedButton` (`/Game/Testin/Blueprints/UI/WBP_MainMenu.SettingsButton` _outputpin) _outputpin)
      (else
        (set `/Game/Testin/Blueprints/UI/WBP_MainMenu._currentSelectedButton` (`/Game/Testin/Blueprints/UI/WBP_MainMenu.QuitButton` _outputpin) _outputpin)))))

(event `Key|Gamepad_DPad_Left`
  (params (Key :type "Key Structure"))
  (:`Pressed`
    (bind _outputpin (`self.MainMenuVisibleCheck`))
    (bind _creditsbutton (`/Game/Testin/Blueprints/UI/WBP_MainMenu.CreditsButton` _outputpin))
    (if (== (`/Game/Testin/Blueprints/UI/WBP_MainMenu._currentSelectedButton` _outputpin) _creditsbutton)
      (set `/Game/Testin/Blueprints/UI/WBP_MainMenu._currentSelectedButton` (`/Game/Testin/Blueprints/UI/WBP_MainMenu.SettingsButton` _outputpin) _outputpin)
      (else
        (set `/Game/Testin/Blueprints/UI/WBP_MainMenu._currentSelectedButton` _creditsbutton _outputpin)))))

(event `Key|Gamepad_DPad_Right`
  (params (Key :type "Key Structure"))
  (bind _mainmenu (`self.MainMenu`))
  (:`Pressed`
    (if (`Widget.IsVisible` (`/Game/Testin/Blueprints/UI/WBP_MainMenu.Settings` _mainmenu))
      (set `/Game/Testin/Blueprints/UI/WBP_MainMenu._currentSelectedButton` (`/Game/Testin/Blueprints/UI/WBP_MainMenu.SettingsBack` _mainmenu) _mainmenu)
      (elif (`Widget.IsVisible` (`/Game/Testin/Blueprints/UI/WBP_MainMenu.Credits` _mainmenu))
        (set `/Game/Testin/Blueprints/UI/WBP_MainMenu._currentSelectedButton` (`/Game/Testin/Blueprints/UI/WBP_MainMenu.CreditsBack` _mainmenu) _mainmenu)
        (else
          (bind _outputpin (`self.MainMenuVisibleCheck`))
          (set `/Game/Testin/Blueprints/UI/WBP_MainMenu._currentSelectedButton` (`/Game/Testin/Blueprints/UI/WBP_MainMenu.ContinueButton` _outputpin) _outputpin))))))

(event `Key|Gamepad_FaceButton_Bottom`
  (params (Key :type "Key Structure"))
  (:`Pressed`
    (bind _outputpin (`self.MainMenuVisibleCheck`))
    (bind __currentselectedbutton (`/Game/Testin/Blueprints/UI/WBP_MainMenu._currentSelectedButton` _outputpin))
    (if (or (== __currentselectedbutton (`/Game/Testin/Blueprints/UI/WBP_MainMenu.NewGameButton` _outputpin)) (== __currentselectedbutton (`/Game/Testin/Blueprints/UI/WBP_MainMenu.ContinueButton` _outputpin)))
      (`/Game/Testin/Blueprints/UI/WBP_MainMenu.StartGame` _outputpin)
      (elif (== (`/Game/Testin/Blueprints/UI/WBP_MainMenu._currentSelectedButton` _outputpin) (`/Game/Testin/Blueprints/UI/WBP_MainMenu.QuitButton` _outputpin))
        (`/Game/Testin/Blueprints/UI/WBP_MainMenu.QuitGameFunction` _outputpin)
        (elif (== (`/Game/Testin/Blueprints/UI/WBP_MainMenu._currentSelectedButton` _outputpin) (`/Game/Testin/Blueprints/UI/WBP_MainMenu.CreditsButton` _outputpin))
          (`/Game/Testin/Blueprints/UI/WBP_MainMenu.CreditsFunction` _outputpin)
          (elif (== (`/Game/Testin/Blueprints/UI/WBP_MainMenu._currentSelectedButton` _outputpin) (`/Game/Testin/Blueprints/UI/WBP_MainMenu.SettingsButton` _outputpin))
            (`/Game/Testin/Blueprints/UI/WBP_MainMenu.SettingsFunction` _outputpin)
            (elif (== (`/Game/Testin/Blueprints/UI/WBP_MainMenu._currentSelectedButton` _outputpin) (`/Game/Testin/Blueprints/UI/WBP_MainMenu.SettingsBack` _outputpin))
              (`/Game/Testin/Blueprints/UI/WBP_MainMenu.SettingsBackFunction` _outputpin)
              (elif (== (`/Game/Testin/Blueprints/UI/WBP_MainMenu._currentSelectedButton` _outputpin) (`/Game/Testin/Blueprints/UI/WBP_MainMenu.CreditsBack` _outputpin))
                (`/Game/Testin/Blueprints/UI/WBP_MainMenu.CreditsBackFunction` _outputpin)))))))))

(event `Key|Gamepad_FaceButton_Right`
  (params (Key :type "Key Structure"))
  (bind _mainmenu (`self.MainMenu`))
  (:`Pressed`
    (if (`Widget.IsVisible` (`/Game/Testin/Blueprints/UI/WBP_MainMenu.Settings` _mainmenu))
      (`/Game/Testin/Blueprints/UI/WBP_MainMenu.SettingsBackFunction` _mainmenu)
      (elif (`Widget.IsVisible` (`/Game/Testin/Blueprints/UI/WBP_MainMenu.Credits` _mainmenu))
        (`/Game/Testin/Blueprints/UI/WBP_MainMenu.CreditsBackFunction` _mainmenu)))))

(fn `MainMenuVisibleCheck`
  (returns (OutputPin :type "/Game/Testin/Blueprints/UI/WBP_MainMenu Object Reference"))
  (bind _mainmenu (`self.MainMenu`))
  (if (`Widget.IsVisible` (`/Game/Testin/Blueprints/UI/WBP_MainMenu.MainMenu` _mainmenu))
    (return _mainmenu)))

(fn `UserConstructionScript`)