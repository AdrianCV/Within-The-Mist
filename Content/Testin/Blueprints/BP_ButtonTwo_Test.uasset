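; Test button actor that toggles a linked platform between its start position and a destination actor's location.
; While the test character overlaps its box, pressing E flips the pressed state through a FlipFlop.
; Tick moves the platform in a straight line at constant speed toward the active target, returning at half speed and stopping within a small tolerance.
; Platform rotation interpolation nodes are present but unused.
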(event `self.ReceiveBeginPlay`
  (`self.EnableInput` (`GameplayStatics.GetPlayerController` 0))
  (set `self._startPos` (`self.K2_GetActorLocation` (`self.platform`))))

(event `self.ReceiveTick`
  (params (DeltaSeconds :type "Float (single-precision)"))
  (bind _platform (`self.platform`))
  (bind _platform_2 (`self.platform`))
  (bind (_returnvalue_location _returnvalue_rotation _returnvalue_scale) (`KismetMathLibrary.BreakTransform` (`self.GetTransform` _platform)))
  (bind (_returnvalue_location_2 _returnvalue_rotation_2 _returnvalue_scale_2) (`KismetMathLibrary.BreakTransform` (`self.GetTransform` _platform_2)))
  (if (`self.hasBeenPressed`)
    (if (not (< (`KismetMathLibrary.VSize` (- (`self.K2_GetActorLocation` (`self.destination`)) (`self.K2_GetActorLocation` (`self.platform`)))) 10.0))
      (`self.K2_SetActorTransform` _platform (`KismetMathLibrary.MakeTransform` (+ _returnvalue_location (* (`KismetMathLibrary.Normal` (- (`self.K2_GetActorLocation` (`self.destination`)) (`self.K2_GetActorLocation` (`self.platform`)))) (* (`GameplayStatics.GetWorldDeltaSeconds`) (`self.platformSpeed`)))) _returnvalue_rotation _returnvalue_scale) false false))
    (elif (not (< (`KismetMathLibrary.VSize` (- (`self._startPos`) (`self.K2_GetActorLocation` (`self.platform`)))) 10.0))
      (`self.K2_SetActorTransform` _platform_2 (`KismetMathLibrary.MakeTransform` (+ _returnvalue_location_2 (* (`KismetMathLibrary.Normal` (- (`self._startPos`) (`self.K2_GetActorLocation` (`self.platform`)))) (* (`GameplayStatics.GetWorldDeltaSeconds`) (/ (`self.platformSpeed`) 2.0)))) _returnvalue_rotation_2 _returnvalue_scale_2) false false))))

(event `self.Box.OnComponentBeginOverlap`
  (params (OverlappedComponent :type "PrimitiveComponent Object Reference") (OtherActor :type "Actor Object Reference") (OtherComp :type "PrimitiveComponent Object Reference") (OtherBodyIndex :type Integer) (bFromSweep :type Boolean) (SweepResult :type "HitResult Structure (by ref)"))
  (cast `/Game/Testin/BP_Character_Test` OtherActor)
  (set `self._canBePressed` true))

(event `self.Box.OnComponentEndOverlap`
  (params (OverlappedComponent :type "PrimitiveComponent Object Reference") (OtherActor :type "Actor Object Reference") (OtherComp :type "PrimitiveComponent Object Reference") (OtherBodyIndex :type Integer))
  (cast `/Game/Testin/BP_Character_Test` OtherActor)
  (set `self._canBePressed` false))

(event `Key|E` :consume false
  (params (Key :type "Key Structure"))
  (:`Pressed`
    (if (`self._canBePressed`)
      (`/Engine/EditorBlueprintResources/StandardMacros.FlipFlop`
        (:`A`
          (set `self.hasBeenPressed` true))
        (:`B`
          (set `self.hasBeenPressed` false))))))

(fn `UserConstructionScript`)