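; A test playground button that opens an assigned door when the player character presses Interact inside its box trigger.
; Box overlaps with BP_Character_Test set whether the button can be pressed, and a press latches it on and teleports the player back to their BeginPlay location.
; Once pressed, Tick eases the door toward its start position plus an offset, scaled by speed and delta time.
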(event `self.ReceiveBeginPlay`
  (bind _doortoopen (`self.doorToOpen`))
  (`self.EnableInput` (`GameplayStatics.GetPlayerController` 0))
  (set `self.startPosition` (`self.K2_GetActorLocation` (`GameplayStatics.GetPlayerCharacter` 0)))
  (`/Engine/EditorBlueprintResources/StandardMacros.IsValid` _doortoopen
    (:`Is Valid`
      (set `self.doorStartPos` (`self.K2_GetActorLocation` _doortoopen)))))

(event `self.ReceiveTick`
  (params (DeltaSeconds :type "Float (single-precision)"))
  (bind _doortoopen (`self.doorToOpen`))
  (bind _returnvalue (`self.K2_GetActorLocation` _doortoopen))
  (if (`self.buttonPressed`)
    (`self.K2_SetActorLocation` _doortoopen (+ _returnvalue (* (- (+ (`self.doorNewPos`) (`self.doorStartPos`)) _returnvalue) (* (`self.doorSpeed`) (`GameplayStatics.GetWorldDeltaSeconds`)))) false false)))

(event `self.Box.OnComponentBeginOverlap`
  (params (OverlappedComponent :type "PrimitiveComponent Object Reference") (OtherActor :type "Actor Object Reference") (OtherComp :type "PrimitiveComponent Object Reference") (OtherBodyIndex :type Integer) (bFromSweep :type Boolean) (SweepResult :type "HitResult Structure (by ref)"))
  (cast `/Game/Testin/BP_Character_Test` OtherActor)
  (set `self.canPressButton` true))

(event `self.Box.OnComponentEndOverlap`
  (params (OverlappedComponent :type "PrimitiveComponent Object Reference") (OtherActor :type "Actor Object Reference") (OtherComp :type "PrimitiveComponent Object Reference") (OtherBodyIndex :type Integer))
  (cast `/Game/Testin/BP_Character_Test` OtherActor)
  (set `self.canPressButton` false))

(event `InputAction|Interact`
  (params (Key :type "Key Structure"))
  (:`Pressed`
    (if (`self.canPressButton`)
      (set `self.buttonPressed` true)
      (`self.K2_SetActorLocation` (`GameplayStatics.GetPlayerCharacter` 0) (`self.startPosition`) false false))))

(fn `UserConstructionScript`)