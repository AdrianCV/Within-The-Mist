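; Test elevator button actor that the player holds with the E key while standing in its trigger box.
; Box overlaps with BP_Character_Test set CanBePressed, and E sets IsBeingPressed only while IsActive is also true, clearing it on release or exit.
; Input is enabled directly on the actor, Tick prints a one-time activation message, and pressing while inactive prints a locked message.
; Nothing here sets IsActive or moves an elevator.
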(event `self.ReceiveBeginPlay`
  (`self.EnableInput` (`GameplayStatics.GetPlayerController` 0)))

(event `self.ReceiveTick`
  (params (DeltaSeconds :type "Float (single-precision)"))
  (if (`self.isActive`)
    (`/Engine/EditorBlueprintResources/StandardMacros.DoOnce` false
      (:`Completed`
        (`KismetSystemLibrary.PrintString` "Elevator is activated")))))

(event `Key|E` :consume false
  (params (Key :type "Key Structure"))
  (:`Pressed`
    (if (and (`self._canBePressed`) (`self.isActive`))
      (set `self.isBeingPressed` true)
      (elif (`self._canBePressed`)
        (`KismetSystemLibrary.PrintString` "Shits locked yo"))))
  (:`Released`
    (set `self.isBeingPressed` false)))

(event `self.Box.OnComponentBeginOverlap`
  (params (OverlappedComponent :type "PrimitiveComponent Object Reference") (OtherActor :type "Actor Object Reference") (OtherComp :type "PrimitiveComponent Object Reference") (OtherBodyIndex :type Integer) (bFromSweep :type Boolean) (SweepResult :type "HitResult Structure (by ref)"))
  (cast `/Game/Testin/BP_Character_Test` OtherActor)
  (set `self._canBePressed` true))

(event `self.Box.OnComponentEndOverlap`
  (params (OverlappedComponent :type "PrimitiveComponent Object Reference") (OtherActor :type "Actor Object Reference") (OtherComp :type "PrimitiveComponent Object Reference") (OtherBodyIndex :type Integer))
  (cast `/Game/Testin/BP_Character_Test` OtherActor)
  (set `self._canBePressed` false)
  (set `self.isBeingPressed` false))

(fn `UserConstructionScript`)