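; AC_Trail_Test is a component that gives its owning Character a forward blink with Niagara effects at both ends.
; BeginPlay casts and caches the owner as a Character.
; TrailStart spawns a start effect at the capsule, moves the capsule forward by TrailDistance, then spawns an end effect where it lands.
; The move is an instant swept SetWorldLocation, so blocking geometry cuts it short.
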(event `self.ReceiveBeginPlay`
  (`|ExecutionSequence`
    (:`then_0`
      (bind _ascharacter (cast `Character` (`self.GetOwner`)))
      (set `self.As Character` _ascharacter))))

(event `Trail Start`
  (bind _capsulecomponent (`Character.CapsuleComponent` (`self.As Character`)))
  (bind _returnvalue (`SceneComponent.K2_GetComponentLocation` _capsulecomponent))
  (`NiagaraFunctionLibrary.SpawnSystemAtLocation` "/Game/Testin/VFX/NS_StartTrail.NS_StartTrail" _returnvalue)
  (`SceneComponent.K2_SetWorldLocation` _capsulecomponent (+ _returnvalue (* (`SceneComponent.GetForwardVector` _capsulecomponent) (`self.Trail Distance`))) true false)
  (`NiagaraFunctionLibrary.SpawnSystemAtLocation` "/Game/Testin/VFX/NS_End_Trail.NS_End_Trail" (`SceneComponent.K2_GetComponentLocation` (`Character.CapsuleComponent` (`self.As Character`)))))