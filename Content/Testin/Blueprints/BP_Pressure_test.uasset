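; Test pressure plate that raises a linked actor while pressed and lowers it back when released.
; Overlaps from actors tagged TriggerPressurePlate play or reverse a timeline that moves the switch mesh and set up/down flags.
; Tick uses those flags to VInterpTo the target actor between its BeginPlay position and a configurable height above it.
; Any tagged actor leaving reverses the plate, as overlaps are not counted.
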(event `self.ReceiveBeginPlay`
  (set `self._startPos` (`self.K2_GetActorLocation` (`self.actorToMove`))))

(event `self.ReceiveActorBeginOverlap`
  (params (OtherActor :type "Actor Object Reference"))
  (if (`self.ActorHasTag` OtherActor "TriggerPressurePlate")
    (set `self._goUp` true)
    (set `self._goDown` false)
    (bind (_direction _switchposition) (`Timeline|SwitchActivate` :!label _label)
      (:`Update`
        (`SceneComponent.K2_SetRelativeLocation` (`self.Switch`) (`KismetMathLibrary.MakeVector` 0.0 0.0 _switchposition) false false)))))

(event `self.ReceiveActorEndOverlap`
  (params (OtherActor :type "Actor Object Reference"))
  (if (`self.ActorHasTag` OtherActor "TriggerPressurePlate")
    (set `self._goUp` false)
    (set `self._goDown` true)
    (goto _label :!via `Reverse`)))

(event `self.ReceiveTick`
  (params (DeltaSeconds :type "Float (single-precision)"))
  (bind _actortomove (`self.actorToMove`))
  (bind _actortomove_2 (`self.actorToMove`))
  (if (`self._goUp`)
    (`self.K2_SetActorLocation` _actortomove (`KismetMathLibrary.VInterpTo` (`self.K2_GetActorLocation` _actortomove) (`KismetMathLibrary.MakeVector` (.x (`self._startPos`)) (.y (`self._startPos`)) (+ (.z (`self._startPos`)) (`self.heightToMove`))) (`GameplayStatics.GetWorldDeltaSeconds`) (`self.speed`)) false false)
    (elif (`self._goDown`)
      (`self.K2_SetActorLocation` _actortomove_2 (`KismetMathLibrary.VInterpTo` (`self.K2_GetActorLocation` _actortomove_2) (`self._startPos`) (`GameplayStatics.GetWorldDeltaSeconds`) (`self.speed`)) false false))))

(fn `UserConstructionScript`)