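; BP_Enemy_Test is a test enemy that rises from its spawn point and snaps onto the player.
; While RiseUp is set, Tick interpolates it 150 units upward, then near the top latches AttackingPlayer and teleports it once to the player's location.
; Otherwise, unless attacking, it eases back to its start.
; Sphere overlaps register it in BP_Character_Test's EnemiesInRange; leaving removes it and clears RiseUp, which this graph never sets true.
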(event `self.ReceiveBeginPlay`
  (bind _output_get (set `self._startPos` (`self.K2_GetActorLocation`)))
  (set `self._endPos` (+ _output_get (0.0 0.0 150.0))))

(event `self.ReceiveTick`
  (params (DeltaSeconds :type "Float (single-precision)"))
  (bind _returnvalue (`self.K2_GetActorLocation`))
  (bind _returnvalue_2 (`GameplayStatics.GetWorldDeltaSeconds`))
  (bind __endpos (`self._endPos`))
  (bind _returnvalue_3 (not (`self._attackingPlayer`)))
  (if (and (`self.riseUp`) _returnvalue_3)
    (`self.K2_SetActorLocation` (`KismetMathLibrary.VInterpTo` _returnvalue __endpos _returnvalue_2 0.5))
    (if (== _returnvalue __endpos :`ErrorTolerance` 10.0)
      (set `self._attackingPlayer` true)
      (`self.K2_SetActorLocation` (`self.K2_GetActorLocation` (`GameplayStatics.GetPlayerCharacter` 0))))
    (elif _returnvalue_3
      (`self.K2_SetActorLocation` (`KismetMathLibrary.VInterpTo` _returnvalue (`self._startPos`) _returnvalue_2 0.5)))))

(event `self.Sphere.OnComponentBeginOverlap`
  (params (OverlappedComponent :type "PrimitiveComponent Object Reference") (OtherActor :type "Actor Object Reference") (OtherComp :type "PrimitiveComponent Object Reference") (OtherBodyIndex :type Integer) (bFromSweep :type Boolean) (SweepResult :type "HitResult Structure (by ref)"))
  (bind _asbp_character_test (cast `/Game/Testin/BP_Character_Test` OtherActor))
  (`KismetArrayLibrary.Array_Add` (`/Game/Testin/BP_Character_Test.enemiesInRange` _asbp_character_test) self))

(event `self.Sphere.OnComponentEndOverlap`
  (params (OverlappedComponent :type "PrimitiveComponent Object Reference") (OtherActor :type "Actor Object Reference") (OtherComp :type "PrimitiveComponent Object Reference") (OtherBodyIndex :type Integer))
  (bind _asbp_character_test (cast `/Game/Testin/BP_Character_Test` OtherActor))
  (`KismetArrayLibrary.Array_RemoveItem` (`/Game/Testin/BP_Character_Test.enemiesInRange` _asbp_character_test) self)
  (set `self.riseUp` false))

(fn `UserConstructionScript`)