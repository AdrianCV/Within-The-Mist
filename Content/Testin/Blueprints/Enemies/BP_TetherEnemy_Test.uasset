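; Test tether enemy that chases a BP_Character_Test within a maximum distance of its starting position.
; RangeCol overlaps track the player; after a delay, Tick moves the enemy toward them at Speed in XY while height eases via FInterpTo.
; Losing the player sends it back toward the start; exceeding the leash also resets the delay, which restarts if the player remains in range.
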(event `self.ReceiveBeginPlay`
  (set `self._startPos` (`self.K2_GetActorLocation`)))

(event `self.ReceiveTick`
  (params (DeltaSeconds :type "Float (single-precision)"))
  (bind _returnvalue (`self.K2_GetActorLocation`))
  (bind _returnvalue_2 (`self.K2_GetActorLocation`))
  (bind _returnvalue_3 (`self.K2_GetActorLocation` (`self._player`)))
  (bind (_returnvalue_x _returnvalue_y) (`KismetMathLibrary.BreakVector` (+ _returnvalue (* (`KismetMathLibrary.Normal` (- _returnvalue_3 _returnvalue)) (* (`GameplayStatics.GetWorldDeltaSeconds`) (`self.speed`))))))
  (if (`self._delayStarted`)
    (if (> (`KismetMathLibrary.Vector_Distance` (`self._startPos`) (`self.K2_GetActorLocation`)) (`self.maxDistanceFromStart`))
      (set `self._delayStarted` false)
      (else
        (set `self._hasReset` false)
        (set `self._delayTime` (+ (`self._delayTime`) (`GameplayStatics.GetWorldDeltaSeconds`)))
        (if (and (>= (`self._delayTime`) (`self.delayDuration`)) (not (`self._hasReset`)))
          (`self.K2_SetActorLocation` (`KismetMathLibrary.MakeVector` _returnvalue_x _returnvalue_y (`KismetMathLibrary.FInterpTo` (.z _returnvalue) (.z _returnvalue_3) (`GameplayStatics.GetWorldDeltaSeconds`) 0.2))))))
    (else
      (set `self._delayTime` 0.0)
      (`self.K2_SetActorLocation` (+ _returnvalue_2 (* (`KismetMathLibrary.Normal` (- (`self._startPos`) _returnvalue_2)) (* (`GameplayStatics.GetWorldDeltaSeconds`) (`self.speed`)))))
      (set `self._hasReset` true)
      (set `self._delayStarted` (`self._playerInRange`)))))

(event `self.Range Col.OnComponentBeginOverlap`
  (params (OverlappedComponent :type "PrimitiveComponent Object Reference") (OtherActor :type "Actor Object Reference") (OtherComp :type "PrimitiveComponent Object Reference") (OtherBodyIndex :type Integer) (bFromSweep :type Boolean) (SweepResult :type "HitResult Structure (by ref)"))
  (bind _asbp_character_test (cast `/Game/Testin/BP_Character_Test` OtherActor))
  (set `self._player` _asbp_character_test)
  (set `self._delayStarted` true)
  (set `self._playerInRange` true))

(event `self.Range Col.OnComponentEndOverlap`
  (params (OverlappedComponent :type "PrimitiveComponent Object Reference") (OtherActor :type "Actor Object Reference") (OtherComp :type "PrimitiveComponent Object Reference") (OtherBodyIndex :type Integer))
  (cast `/Game/Testin/BP_Character_Test` OtherActor)
  (set `self._player` null)
  (set `self._delayStarted` false)
  (set `self._playerInRange` false))

(fn `UserConstructionScript`)