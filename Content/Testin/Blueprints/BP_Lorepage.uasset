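; BP_Lorepage is a lore page pickup actor that shows its text in a UI when the player walks into it.
; On Box overlap by BP_Character_Test, it creates a WBP_LorepageUI widget if none is valid, passing itself and its Text.
; It then adds the widget to the viewport, switches the character to UI via SwapToUI and pauses the game.
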(event `self.Box.OnComponentBeginOverlap`
  (params (OverlappedComponent :type "PrimitiveComponent Object Reference") (OtherActor :type "Actor Object Reference") (OtherComp :type "PrimitiveComponent Object Reference") (OtherBodyIndex :type Integer) (bFromSweep :type Boolean) (SweepResult :type "HitResult Structure (by ref)"))
  (bind _asbp_character_test (cast `/Game/Testin/BP_Character_Test` OtherActor))
  (`/Engine/EditorBlueprintResources/StandardMacros.IsValid` (`self.LoreItem`)
    (:`Is Not Valid`
      (bind _returnvalue (`|CreateWidget` "/Game/Testin/Blueprints/UI/WBP_LorepageUI.WBP_LorepageUI_C"))
      (set `self.LoreItem` _returnvalue)
      (set `/Game/Testin/Blueprints/UI/WBP_LorepageUI.Lorepage` self _returnvalue)
      (set `TextBlock.Text` (`self.Text`) (`/Game/Testin/Blueprints/UI/WBP_LorepageUI.LoreTextbox` _returnvalue))
      (`UserWidget.AddToViewport` _returnvalue 0)
      (`/Game/Testin/BP_Character_Test.SwapToUI` _asbp_character_test)
      (`GameplayStatics.SetGamePaused` true))))

(fn `UserConstructionScript`)