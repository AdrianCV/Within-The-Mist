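; Procedural building Blueprint that lays a ring of random wall, floor, roof or railing meshes along a circular spline, minus optional door spaces.
; The construction script rebuilds the spline from Radius and Segments, using tan-based tangent lengths to approximate a true circle.
; It then adds spline mesh components at mesh-length intervals, picking random variants of the selected piece type and clamping tangents to that length.
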(event EventBeginPlay)

(event Collision|EventActorBeginOverlap
  (params (OtherActor :type Actor%20Object%20Reference)))

(event EventTick
  (params (DeltaSeconds :type Float%20%28single-precision%29)))

(fn ConstructionScript
  ;[1 0.000256 0.05799] Creates a circular spline
  (CallFunction|CircleCreation (Variables|Default|GetCircle%20spline) (Variables|Default|GetRadius) (Variables|Default|GetSegments))
  ;[0.1076 1 0] Gets the spline and divides it with the lenght of the mesh
  (for _index (range 0 (- (Math|Float|Truncate (/ (Spline|GetSplineLength (Variables|Default|GetCircle%20Spline)) (Variables|Default|GetMesh%20Length))) (Variables|Default|GetDoor%20Spaces)))
    (Variables|Default|SetLoop%20Index _index)
    ;[1 0.9262 0] Adds mesh to the spline
    (bind _returnvalue (AddComponent|AddSplineMeshComponent false))
    ;;[1 0 0.9918] Picks between walls, floors, roof, and railing
    (switch int (Math|Integer|Clamp(Integer) (Variables|Default|Get0%20wall%20/%201%20Floor%20/%202%20Roof%20/%203%20Railing) 0 3)
      (:0
        (Variables|Default|SetMesh%20Length 211.0)
        ;;[0 1 0.8645] ADD YOUR OWN. These are the meshes the script picks form
        (Components|StaticMesh|SetStaticMesh _returnvalue (.OutItem (Utilities|Array|Random (Utilities|Array|MakeArray "/Game/Building_Imports/building_meshes/Wall_1.Wall_1" "/Game/Building_Imports/building_meshes/Wall_2.Wall_2" "/Game/Building_Imports/building_meshes/Wall_3.Wall_3")))))
      (:1
        (Variables|Default|SetMesh%20Length 212.0)
        (Components|StaticMesh|SetStaticMesh _returnvalue (.OutItem (Utilities|Array|Random (Utilities|Array|MakeArray "/Game/Building_Imports/building_meshes/Floor_1.Floor_1" "/Game/Building_Imports/building_meshes/Floor_2.Floor_2")))))
      (:2
        (Variables|Default|SetMesh%20Length 212.0)
        (Components|StaticMesh|SetStaticMesh _returnvalue (.OutItem (Utilities|Array|Random (Utilities|Array|MakeArray "/Game/Building_Imports/building_meshes/Roof_1.Roof_1" "/Game/Building_Imports/building_meshes/Roof_2.Roof_2" "/Game/Building_Imports/building_meshes/Roof_3.Roof_3")))))
      (:3
        (Variables|Default|SetMesh%20Length 508.0)
        (Components|StaticMesh|SetStaticMesh _returnvalue (.OutItem (Utilities|Array|Random (Utilities|Array|MakeArray "/Game/Building_Imports/building_meshes/Railing1.Railing1" "/Game/Building_Imports/building_meshes/Railing2.Railing2" "/Game/Building_Imports/building_meshes/Railing3.Railing3"))))))
    ;;[0.03505 0 1] Sets the Posision and tangent of the meshes
    (bind (_pos _tan) (CallFunction|GetStartPos/tan (Variables|Default|GetLoop%20Index)))
    (bind (_pos_2 _tan_2) (CallFunction|GetEndPos/Tan (Variables|Default|GetLoop%20Index)))
    (SplineMesh|SetStartandEnd _returnvalue _pos _tan _pos_2 _tan_2 true :!class /Script/Engine.SplineMeshComponent)
    (Transformation|AttachComponentToComponent _returnvalue (Variables|Default|GetCircle%20spline) "None" "KeepRelative" "KeepRelative" "KeepRelative" true)
    (Collision|SetCollisionEnabled _returnvalue (Variables|Default|GetCollision))))

(fn GetStartPos/tan
  (params (Index :type Integer))
  (bind _mesh_length (Variables|Default|GetMesh%20Length))
  (bind _circle_spline (Variables|Default|GetCircle%20Spline))
  (bind _returnvalue (* Index _mesh_length))
  (return (Spline|GetLocationatDistanceAlongSpline _circle_spline _returnvalue "Local") (Math|Vector|ClampVectorSize (Spline|GetTangentatDistanceAlongSpline _circle_spline _returnvalue "Local") 0.0 (Variables|Default|GetMesh%20Length))))

(fn GetEndPos/Tan
  (params (Index :type Integer))
  (bind _returnvalue (+ Index 1))
  (bind _mesh_length (Variables|Default|GetMesh%20Length))
  (bind _circle_spline (Variables|Default|GetCircle%20Spline))
  (bind _returnvalue_2 (* _returnvalue _mesh_length))
  (return (Spline|GetLocationatDistanceAlongSpline _circle_spline _returnvalue_2 "Local") (Math|Vector|ClampVectorSize (Spline|GetTangentatDistanceAlongSpline _circle_spline _returnvalue_2 "Local") 0.0 (Variables|Default|GetMesh%20Length))))

(fn CircleCreation
  (params (Circle%20spline :type Spline%20Component%20Object%20Reference) (Radius :type Float%20%28double-precision%29) (Segments :type Integer))
  (bind _returnvalue (- Segments 1))
  (Spline|ClearSplinePoints Circle%20spline false)
  (if (> Segments 0)
    (for _index (range 0 _returnvalue)
      (Spline|AddSplinePoint Circle%20spline (Math|Vector|MakeVector (* (Math|Trig|Sin(Degrees) (Math|Float|MapRangeClamped (Math|Conversions|ToFloat(Integer) _index) 0.0 (Math|Conversions|ToFloat(Integer) _returnvalue) 0.0 (Math|Conversions|ToFloat(Integer) (|(360-(360/vSegments)) Segments)))) Radius) (* (Math|Trig|Cos(Degrees) (Math|Float|MapRangeClamped (Math|Conversions|ToFloat(Integer) _index) 0.0 (Math|Conversions|ToFloat(Integer) _returnvalue) 0.0 (Math|Conversions|ToFloat(Integer) (|(360-(360/vSegments)) Segments)))) Radius) 0.0) "Local" true)
      (Spline|SetTangentatSplinePoint Circle%20spline _index (* (Math|Vector|GetRightVector (Math|Rotator|FindLookatRotation (Math|Vector|MakeVector (* (Math|Trig|Sin(Degrees) (Math|Float|MapRangeClamped (Math|Conversions|ToFloat(Integer) _index) 0.0 (Math|Conversions|ToFloat(Integer) _returnvalue) 0.0 (Math|Conversions|ToFloat(Integer) (|(360-(360/vSegments)) Segments)))) Radius) (* (Math|Trig|Cos(Degrees) (Math|Float|MapRangeClamped (Math|Conversions|ToFloat(Integer) _index) 0.0 (Math|Conversions|ToFloat(Integer) _returnvalue) 0.0 (Math|Conversions|ToFloat(Integer) (|(360-(360/vSegments)) Segments)))) Radius) 0.0) (Math|Vector|MakeVector 0.0 0.0 0.0))) (* Radius (|(4*(tan(((D2R((360/vSegments)))/4)))) Segments))) "Local" true)))
  (Spline|UpdateSpline Circle%20spline)
  (return))