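; BP_DockSegment is a spline-driven actor that builds a dock from randomly chosen bridge meshes, with optional railings.
; Its construction script runs a deck pass and a railing pass, each adding deformed spline mesh components with a configurable collision setting.
; Helper functions sample segment endpoints by distance and clamp tangents to the section length.
; Both passes share SectionLength, overwriting it inside their loops with their own mesh length.
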(fn `Get End pos/Tangent`
  (params (Index :type Integer))
  (returns (Position :type "Vector Structure") (Tangent :type "Vector Structure"))
  (bind _spline (`self.Spline`))
  (bind _returnvalue (* (+ Index 1) (`self.Section Length`)))
  (return (`SplineComponent.GetLocationAtDistanceAlongSpline` _spline _returnvalue "Local") (`KismetMathLibrary.ClampVectorSize` (`SplineComponent.GetTangentAtDistanceAlongSpline` _spline _returnvalue "Local") 0.0 (`self.Section Length`))))

(fn `Get Start pos/Tangent`
  (params (Index :type Integer))
  (returns (Position :type "Vector Structure") (Tangent :type "Vector Structure"))
  (bind _spline (`self.Spline`))
  (bind _returnvalue (* Index (`self.Section Length`)))
  (return (`SplineComponent.GetLocationAtDistanceAlongSpline` _spline _returnvalue "Local") (`KismetMathLibrary.ClampVectorSize` (`SplineComponent.GetTangentAtDistanceAlongSpline` _spline _returnvalue "Local") 0.0 (`self.Section Length`))))

(fn `UserConstructionScript`
  (locals (`Loop Index` :type Integer))
  (`|ExecutionSequence`
    (:`then_0`
      (if true
        (for _index (range (`KismetMathLibrary.FTrunc` (/ (`SplineComponent.GetSplineLength` (`self.Spline`)) (`self.Section Length`))))
          (set `local.Loop Index` _index)
          (bind _returnvalue (`AddComponent|NODE_AddSplineMeshComponent-0`))
          (set `self.Section Length` 200.0)
          (`StaticMeshComponent.SetStaticMesh` _returnvalue (`KismetArrayLibrary.Array_Random` (`|MakeArray` "/Game/Building_Imports/dock_meshes/Bridge1.Bridge1" "/Game/Building_Imports/dock_meshes/Bridge2.Bridge2" "/Game/Building_Imports/dock_meshes/Bridge3.Bridge3" :!type "StaticMesh Object Reference")))
          (`SplineMeshComponent.SetForwardAxis` _returnvalue "X" true)
          (bind (_position _tangent) (`self.Get Start pos/Tangent` (`local.Loop Index`)))
          (bind (_position_2 _tangent_2) (`self.Get End pos/Tangent` (`local.Loop Index`)))
          (`SplineMeshComponent.SetStartAndEnd` _returnvalue _position _tangent _position_2 _tangent_2 true)
          (`PrimitiveComponent.SetCollisionEnabled` _returnvalue (`self.Collision Type`)))))
    (:`then_1`
      (if (`self.Railing`)
        (for _index_2 (range (`KismetMathLibrary.FTrunc` (/ (`SplineComponent.GetSplineLength` (`self.Spline`)) (`self.Section Length`))))
          (set `local.Loop Index` _index_2)
          (bind _returnvalue_2 (`AddComponent|NODE_AddSplineMeshComponent-7`))
          (set `self.Section Length` 508.0)
          (`StaticMeshComponent.SetStaticMesh` _returnvalue_2 (`KismetArrayLibrary.Array_Random` (`|MakeArray` "/Game/Building_Imports/building_meshes/Railing1.Railing1" "/Game/Building_Imports/building_meshes/Railing2.Railing2" "/Game/Building_Imports/building_meshes/Railing3.Railing3" :!type "StaticMesh Object Reference")))
          (`SplineMeshComponent.SetForwardAxis` _returnvalue_2 "X" true)
          (bind (_position_3 _tangent_3) (`self.Get Start pos/Tangent` (`local.Loop Index`)))
          (bind (_position_4 _tangent_4) (`self.Get End pos/Tangent` (`local.Loop Index`)))
          (`SplineMeshComponent.SetStartAndEnd` _returnvalue_2 _position_3 _tangent_3 _position_4 _tangent_4 true)
          (`PrimitiveComponent.SetCollisionEnabled` _returnvalue_2 (`self.Collision Type`)))))))